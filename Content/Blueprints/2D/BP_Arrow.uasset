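; BP_Arrow is a 2D Paper sprite arrow projectile that launches itself forward with a physics impulse on BeginPlay.
; A timeline blends the sprite's pitch toward a downward angle during flight to tilt the arrow.
; Check re-calls itself on a short delay, sphere-tracing on Visibility at the Sphere component with debug drawing.
; On a hit it disables physics and stops the timeline, freezing the arrow in place.
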(event Custom|Check
  (bind _sphere (Variables|Default|GetSphere))
  (bind _returnvalue (Transformation|GetWorldLocation _sphere))
  (if (not (Variables|Default|GetHit))
    (bind _returnvalue_2 (Collision|SphereTraceByChannel _returnvalue _returnvalue 1e+01 "TraceTypeQuery1" false 0 "ForDuration"))
    (bind _output_get (Variables|Default|SetHit _returnvalue_2))
    (if _output_get
      (Physics|SetSimulatePhysics (Variables|Default|GetPaperSprite) false)
      (CallFunction|StopArrow)
      (else
        (Utilities|FlowControl|Delay 0.2)
        (CallFunction|Check)))))

(event Custom|ArrowAnim
  (bind _papersprite (Variables|Default|GetPaperSprite))
  (bind _returnvalue (Transformation|GetWorldRotation _papersprite))
  (bind (_roll _pitch _yaw) (Math|Rotator|BreakRotator _returnvalue))
  (bind _alpha (Timeline|Timeline PlayFromStart)
    (:Update
      (Transformation|SetWorldRotation (Variables|Default|GetPaperSprite) (Math|Rotator|Lerp(Rotator) _returnvalue (Math|Rotator|MakeRotator _roll -3e+01 _yaw) _alpha) false false))))

(event Custom|StopArrow
  (bind _papersprite (Variables|Default|GetPaperSprite))
  (bind _returnvalue (Transformation|GetWorldRotation _papersprite))
  (bind (_roll _pitch _yaw) (Math|Rotator|BreakRotator _returnvalue))
  (bind _alpha (Timeline|Timeline Stop)
    (:Update
      (Transformation|SetWorldRotation (Variables|Default|GetPaperSprite) (Math|Rotator|Lerp(Rotator) _returnvalue (Math|Rotator|MakeRotator _roll -3e+01 _yaw) _alpha) false false))))

(event EventBeginPlay
  (bind _papersprite (Variables|Default|GetPaperSprite))
  (Physics|AddImpulse _papersprite (* (Math|Vector|GetForwardVector _papersprite) 1e+03) "None" true)
  (CallFunction|ArrowAnim)
  (CallFunction|Check))

(fn ConstructionScript)