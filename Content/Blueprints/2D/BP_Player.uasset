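; Player character for a 2D side-scrolling platformer, with Enhanced Input movement, a bow attack and a dash.
; Tick grid-snaps the spring arm for a pixel-perfect camera and flips control rotation to face horizontal velocity.
; Jump, ledge and landing events drive animation nodes; attacking plays an override with backward recoil, while the Shoot flag blocks other actions except the dash.
; SpawnArrow fires BP_Arrow with camera shake; Q dashes forward with effects and a cooldown.
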(event Custom|SpawnArrow
  (Game|SpawnActorfromClass "/Game/Blueprints/2D/BP_Arrow.BP_Arrow_C" (Transformation|GetActorTransform) "Undefined" "MultiplyWithRoot" 0 0)
  (Camera|PlayWorldCameraShake "/Game/Blueprints/2D/BP_CameraShake.BP_CameraShake_C" (Transformation|GetWorldLocation (Variables|Default|GetCamera)) 0.0 1e+02 5.0 true))

(event Input|EnhancedActionEvents|EnhancedInputActionIA_Jump
  (params (ActionValue :type Boolean) (ElapsedSeconds :type Float%20%28double-precision%29) (TriggeredSeconds :type Float%20%28double-precision%29) (InputAction :type Input%20Action%20Object%20Reference :default "/Game/ThirdPerson/Input/Actions/IA_Jump.IA_Jump"))
  (:Started
    (if (not (Variables|Default|GetShoot))
      (Class|PaperZDAnimInstance|JumptoNode (Variables|/Script/PaperZD.PaperZDAnimationComponent|GetAnimInstance (Variables|Default|GetAnimationComponent)) "Airborne" "None"))))

(event Input|EnhancedActionEvents|EnhancedInputActionIA_Move2D
  (params (ActionValue :type Float%20%28double-precision%29) (ElapsedSeconds :type Float%20%28double-precision%29) (TriggeredSeconds :type Float%20%28double-precision%29) (InputAction :type Input%20Action%20Object%20Reference :default "/Game/ThirdPerson/Input/Actions/IA_Move2D.IA_Move2D"))
  (:Triggered
    (if (not (Variables|Default|GetShoot))
      (Pawn|Input|AddMovementInput "1.000000,0.000000,0.000000" ActionValue false))))

(event Input|EnhancedActionEvents|EnhancedInputActionIA_Attack
  (params (ActionValue :type Boolean) (ElapsedSeconds :type Float%20%28double-precision%29) (TriggeredSeconds :type Float%20%28double-precision%29) (InputAction :type Input%20Action%20Object%20Reference :default "/Game/ThirdPerson/Input/Actions/IA_Attack.IA_Attack"))
  (bind _returnvalue (Transformation|GetActorForwardVector))
  (:Triggered
    (if (not (Variables|Default|GetShoot))
      (bind _animationlength (Class|PaperZDAnimInstance|PlayAnimationOverride (Variables|/Script/PaperZD.PaperZDAnimationComponent|GetAnimInstance (Variables|Default|GetAnimationComponent)) "/Game/Assets/PaperAssets/AnimSequences/Shoot.Shoot" "Shoot" 1.0 0.0))
      (Utilities|FlowControl|Sequence
        (:then_0
          (Utilities|FlowControl|Delay _animationlength)
          (Variables|Default|SetShoot false))
        (:then_1
          (Variables|Default|SetShoot true)
          (|AsyncRootMovement (Variables|Character|GetCharacterMovement) (Math|Vector|MakeVector (* (.x _returnvalue) -1.0) (.y _returnvalue) (.z _returnvalue)) 1.5e+02 0.0 false 0 "MaintainLastRootMotionVelocity" "0, 0, 0" 0.0 true))))))

(event EventTick
  (params (DeltaSeconds :type Float%20%28single-precision%29))
  (bind _returnvalue (Transformation|GetActorLocation))
  (bind _returnvalue_2 (Pawn|GetController))
  (bind _returnvalue_3 (Pawn|GetController))
  ;[1 1 1] Snap the SpringArm(Pixel Perfect Effect)
  (Transformation|SetWorldLocation (Variables|Default|GetSpringArm) (Math|Vector|MakeVector (Math|Float|SnapToGrid(Float) (.x _returnvalue) 3.333333) 0.0 (Math|Float|SnapToGrid(Float) (.z _returnvalue) 3.333333)) false false)
  (if (not (Variables|Default|GetShoot))
    ;[1 0.6093 0] Check Direction
    (Math|Float|CompareFloat (.X (Math|Vector|BreakVector (Variables|/Script/Engine.MovementComponent|GetVelocity (Pawn|GetMovementComponent)))) 0.0
      (:>
        ;[0.4845 0.2088 1] Look Right
        (Utilities|IsValid _returnvalue_3
          (:Is%20Valid
            (Pawn|SetControlRotation _returnvalue_3 (Math|Rotator|MakeRotator 0.0 0.0 0.0)))))
      (:<
        ;[0.4845 0.2088 1] Look Left
        (Utilities|IsValid _returnvalue_2
          (:Is%20Valid
            (Pawn|SetControlRotation _returnvalue_2 (Math|Rotator|MakeRotator 0.0 0.0 1.8e+02))))))))

(event EventOnWalkingOffLedge
  (params (PreviousFloorImpactNormal :type Vector%20%28by%20ref%29 :default "0, 0, 0") (PreviousFloorContactNormal :type Vector%20%28by%20ref%29 :default "0, 0, 0") (PreviousLocation :type Vector%20%28by%20ref%29 :default "0, 0, 0") (TimeDelta :type Float%20%28single-precision%29))
  (if (not (Variables|Default|GetShoot))
    (Class|PaperZDAnimInstance|JumptoNode (Variables|/Script/PaperZD.PaperZDAnimationComponent|GetAnimInstance (Variables|Default|GetAnimationComponent)) "Airborne" "None")))

(event EventBeginPlay
  (bind _asplayer_controller (Utilities|Casting|CastToPlayerController (Pawn|GetController)))
  (Input|AddMappingContext (PlayerController|LocalPlayerSubsystems|GetEnhancedInputLocalPlayerSubsystem _asplayer_controller) "/Game/ThirdPerson/Input/ICM_Platformer.ICM_Platformer" 0 "(bIgnoreAllPressedKeysUntilRelease=True,bForceImmediately=False)"))

(event EventOnLanded
  (params (Hit :type Hit%20Result%20Structure%20%28by%20ref%29))
  (Class|PaperZDAnimInstance|JumptoNode (Variables|/Script/PaperZD.PaperZDAnimationComponent|GetAnimInstance (Variables|Default|GetAnimationComponent)) "Landed" "None"))

(event Input|KeyboardEvents|Q
  (params (Key :type Key%20Structure :default "None"))
  (:Pressed
    (if (not (Variables|Default|GetPower))
      (Niagara|SpawnSystematLocation "/Game/Niagara/Arrow/NS_Arrow.NS_Arrow" (Transformation|GetActorLocation))
      (|AsyncRootMovement (Variables|Character|GetCharacterMovement) (Transformation|GetActorForwardVector) 1e+03 0.4 false 0 "ClampVelocity" "0, 0, 0" 0.0 false
        (:then
          (Variables|Default|SetPower true)
          (Camera|PlayWorldCameraShake "/Game/Blueprints/2D/BP_CameraShake.BP_CameraShake_C" (Transformation|GetWorldLocation (Variables|Default|GetCamera)) 0.0 1e+02 5.0 true))
        (:OnComplete
          (Utilities|FlowControl|Delay 2.0)
          (Variables|Default|SetPower false))))))

(fn ConstructionScript)